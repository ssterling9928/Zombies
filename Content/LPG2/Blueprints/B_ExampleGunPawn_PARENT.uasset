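; Parent pawn for example modular guns, assembled from separate part components such as receiver, barrel, grip, stock, magazine, sight, muzzle brake and attachments.
; The Construction Script copies mesh variables onto each component, so different variable values yield different gun builds.
; Grip, stock and every attachment slot have paired skeletal (M) and static (S) mesh components.
; The event graph holds only disabled placeholder events, with no runtime logic.
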(event EventBeginPlay)

(event Collision|EventActorBeginOverlap
  (params (OtherActor :type Actor%20Object%20Reference)))

(event EventTick
  (params (DeltaSeconds :type Float%20%28single-precision%29)))

(fn ConstructionScript
  (Class|SkinnedMeshComponent|SetSkeletalMesh (Variables|Default|GetGripM) (Variables|BaseGunParts|GetGripMeshM) true)
  (Components|StaticMesh|SetStaticMesh (Variables|Default|GetGripS) (Variables|BaseGunParts|GetGripMeshS))
  (Class|SkinnedMeshComponent|SetSkeletalMesh (Variables|Default|GetReciever) (Variables|BaseGunParts|GetRecieverMesh) true)
  (Class|SkinnedMeshComponent|SetSkeletalMesh (Variables|Default|GetBarrel) (Variables|BaseGunParts|GetBarrelMesh) true)
  (Class|SkinnedMeshComponent|SetSkeletalMesh (Variables|Default|GetStockM) (Variables|BaseGunParts|GetStockMeshM) true)
  (Components|StaticMesh|SetStaticMesh (Variables|Default|GetStockS) (Variables|BaseGunParts|GetStockMeshS))
  (Class|SkinnedMeshComponent|SetSkeletalMesh (Variables|Default|GetAttachmentM) (Variables|BaseGunParts|GetAttachmentMeshM) true)
  (Components|StaticMesh|SetStaticMesh (Variables|Default|GetAttachmentS) (Variables|BaseGunParts|GetAttachmentMeshS))
  (Components|StaticMesh|SetStaticMesh (Variables|Default|GetMag) (Variables|BaseGunParts|GetMagMesh))
  (Components|StaticMesh|SetStaticMesh (Variables|Default|GetSight) (Variables|BaseGunParts|GetSightMesh))
  (Class|SkinnedMeshComponent|SetSkeletalMesh (Variables|Default|GetBAttachmentM) (Variables|BarrelParts|GetBAttachmentMeshM) true)
  (Components|StaticMesh|SetStaticMesh (Variables|Default|GetBAttachmentS) (Variables|BarrelParts|GetBAttachmentMeshS))
  (Class|SkinnedMeshComponent|SetSkeletalMesh (Variables|Default|GetRAttachmentM) (Variables|BarrelParts|GetRAttachmentMeshM) true)
  (Components|StaticMesh|SetStaticMesh (Variables|Default|GetRAttachmentS) (Variables|BarrelParts|GetRAttachmentMeshS))
  (Class|SkinnedMeshComponent|SetSkeletalMesh (Variables|Default|GetTAttachmentM) (Variables|BarrelParts|GetTAttachmentMeshM) true)
  (Components|StaticMesh|SetStaticMesh (Variables|Default|GetTAttachmentS) (Variables|BarrelParts|GetTAttachmentMeshS))
  (Class|SkinnedMeshComponent|SetSkeletalMesh (Variables|Default|GetLAttachmentM) (Variables|BarrelParts|GetLAttachmentMeshM) true)
  (Components|StaticMesh|SetStaticMesh (Variables|Default|GetLAttachmentS) (Variables|BarrelParts|GetLAttachmentMeshS))
  (Components|StaticMesh|SetStaticMesh (Variables|Default|GetMuzzleBreak) (Variables|BarrelParts|GetMuzzleBreakMesh)))